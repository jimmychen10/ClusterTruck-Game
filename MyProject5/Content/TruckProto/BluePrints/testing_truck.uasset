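; Prototype truck actor that travels along the level's Spline_path_BP spline over a set duration.
; On BeginPlay it finds the spline actor and plays a timeline with rate scaled by TimeToComplete, setting world location and local-space spline rotation by distance.
; A separate GetPath function, uncalled here, maps yaw toward ActivePath's closest point to a clamped steering-style value, with its tangent look-ahead zeroed.
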(event Custom|Move%20Object
  (bind _spline_ref (Variables|Default|GetSpline%20REF))
  (bind _spline (Variables|/Game/TruckProto/BluePrints/Spline_path_BP.Spline_path_BP_C|GetSpline _spline_ref))
  (Components|Timeline|SetPlayRate (Variables|Default|GetMove%20Obect%20T) (/ 1.0 (Variables|Default|Gettime%20to%20complete)))
  (bind _move_track (Timeline|Move%20Obect%20T Play)
    (:Update
      (Transformation|SetActorTransform (Math|Transform|MakeTransform (Spline|GetLocationatDistanceAlongSpline _spline (Math|Float|Lerp 0.0 (Spline|GetSplineLength (Variables|/Game/TruckProto/BluePrints/Spline_path_BP.Spline_path_BP_C|GetSpline (Variables|Default|GetSpline%20REF))) _move_track) "World") (Spline|GetRotationatDistanceAlongSpline _spline (Math|Float|Lerp 0.0 (Spline|GetSplineLength (Variables|/Game/TruckProto/BluePrints/Spline_path_BP.Spline_path_BP_C|GetSpline (Variables|Default|GetSpline%20REF))) _move_track) "Local") "1.000000,1.000000,1.000000")))))

(event EventBeginPlay
  (bind _returnvalue (Actor|GetActorOfClass "/Game/TruckProto/BluePrints/Spline_path_BP.Spline_path_BP_C"))
  (Variables|Default|SetSpline%20REF _returnvalue)
  (CallFunction|MoveObject))

(fn ConstructionScript)

(fn GetPath
  (bind _returnvalue (Transformation|GetActorLocation))
  (bind _active_path (Variables|Default|GetActive_path))
  (bind _spline (Variables|/Game/TruckProto/BluePrints/Spline_path_BP.Spline_path_BP_C|GetSpline _active_path))
  (return (Math|Float|MapRangeClamped (.yaw (Math|Rotator|Delta(Rotator) (Math|Rotator|FindLookatRotation _returnvalue (Spline|FindLocationClosesttoWorldLocation _spline (+ (* (Math|Vector|Normalize (Class|SplineComponent|FindTangentClosesttoWorldLocation _spline _returnvalue "World")) "") _returnvalue) "World")) (Transformation|GetActorRotation))) -9e+01 9e+01 -1.0 1.0)))